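; BP_BaseWeapon is a base gun Blueprint that handles shooting, ammo and reloading for the player's BP_Hero.
; Shoot checks CanShoot, then spends a round, line-traces from the hero's camera with debug drawing and spawns an attached muzzle flash.
; Reload refills the magazine from spare ammo, limited by capacity.
; Trace hits are unused, PlayShotSound and UpdateGM are empty events, and IsReloading is read but never set here.
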(event `self.ReceiveBeginPlay`
  (bind _asbp_hero (cast `/Game/Character/BP_Hero` (`GameplayStatics.GetPlayerCharacter` 0)))
  (set `self.Character` _asbp_hero)
  (bind _asbp_gm (cast `/Game/BP_GM` (`GameplayStatics.GetGameMode`)))
  (set `self.BP_GM` _asbp_gm))

(event `Shoot`
  (bind _result (`self.CanShoot`))
  (if _result
    (`self.ReduceAmmo`)
    (`self.CreateShotTrace` 10000.0)
    (`self.CreateMuzzleFlash`)
    (`self.PlayShotSound`)))

(event `ReduceAmmo`
  (if (> (`self.Ammo`) 0)
    (`/Engine/EditorBlueprintResources/StandardMacros.DecrementInt` (`self.Ammo`)
      (:`  `
        (`self.UpdateGM`)))))

(event `CreateShotTrace`
  (params (Range :type "Float (double-precision)" :default 10000.0))
  (bind _camera (`/Game/Character/BP_Hero.Camera` (`self.Character`)))
  (bind _returnvalue (`SceneComponent.K2_GetComponentLocation` _camera))
  (bind _returnvalue_2 (`KismetMathLibrary.GetForwardVector` (`SceneComponent.K2_GetComponentRotation` _camera)))
  (`KismetSystemLibrary.LineTraceMultiForObjects` :`Start` (+ (* _returnvalue_2 150) _returnvalue) :`End` (+ _returnvalue (* _returnvalue_2 Range)) :`ObjectTypes` (`|MakeArray` "ObjectTypeQuery1" :!type "EObjectTypeQuery Enum") :`DrawDebugType` "ForDuration"))

(event `CreateMuzzleFlash`
  (`GameplayStatics.SpawnEmitterAttached` "/Game/Realistic_Starter_VFX_Pack_Vol2/Particles/Explosion/P_Explosion_Big_A.P_Explosion_Big_A" (`self.Arrow`) "None" (0.0 0.0 0.0) (struct) (0.03 0.03 0.03)))

(event `PlayShotSound`)

(event `UpdateGM`)

(event `Reload`
  (bind _result (`self.CanReload`))
  (if _result
    (bind _output_get (set `self.AmmoToReload` (`KismetMathLibrary.Min` (`self.SpareAmmo`) (- (`self.Capacity`) (`self.Ammo`)))))
    (set `self.Ammo` (+ _output_get (`self.Ammo`)))
    (set `self.SpareAmmo` (- (`self.SpareAmmo`) _output_get))
    (`self.UpdateGM`)))

(fn `CanReload`
  (returns (Result :type Boolean))
  (return (and (> (`self.SpareAmmo`) 0) (< (`self.Ammo`) (`self.Capacity`)))))

(fn `CanShoot`
  (returns (Result :type Boolean))
  (return (and (> (`self.Ammo`) 0) (not (`self.IsReloading`)))))

(fn `UserConstructionScript`)