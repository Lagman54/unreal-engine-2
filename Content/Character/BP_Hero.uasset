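; Player hero character with Enhanced Input movement, sprinting, aiming and pistol/rifle combat, plus HUD and aim widgets.
; Aiming slows to walk, locks rotation to the controller, zooms the spring arm via timeline and permits shooting.
; Weapon switching destroys the current weapon actor and spawns the next on a mesh socket.
; Reload montage completion refills the weapon; only the BeginPlay weapon's NeedReload event is bound, and Tick clamps pitch.
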(event `self.ReceiveBeginPlay`
  ; Event BeginPlay
  (`EnhancedInputSubsystemInterface.AddMappingContext` (pcsubsystem `EnhancedInputLocalPlayerSubsystem` (`GameplayStatics.GetPlayerController` 0)) "/Game/Character/Input/IMC_Player.IMC_Player" 0 (struct))
  (bind _returnvalue (`|CreateWidget` "/Game/UI/WBP_Aim.WBP_Aim_C"))
  (bind _output_get (set `self.AimWidget` _returnvalue))
  (`Widget.SetVisibility` _output_get "Hidden")
  (bind _returnvalue_2 (`|CreateWidget` "/Game/UI/WBP_HUD.WBP_HUD_C"))
  (`UserWidget.AddToViewport` _returnvalue_2 0)
  (`UserWidget.AddToViewport` (`self.AimWidget`) 0)
  (bind _output_get_2 (set `self.CurrentWeaponIndex` 1))
  (`self.Switch Weapon` _output_get_2)
  (add `/Game/Blueprints/Weapons/BP_BaseWeapon.NeedReload` (`self.CurrentWeaponBP`) (delegate `ReloadGun`)))

(event `ReloadGun`
  ; Event BeginPlay
  (if (not (`/Game/Blueprints/Weapons/BP_BaseWeapon.IsReloading` (`self.CurrentWeaponBP`)))
    (bind _result (`/Game/Blueprints/Weapons/BP_BaseWeapon.CanReload` (`self.CurrentWeaponBP`)))
    (if _result
      (`self.PlayReloadAnim`))))

(event `PlayReloadAnim`
  (bind _currentweaponbp (`self.CurrentWeaponBP`))
  (`|PlayMontage` (`self.Mesh`) "/Game/Animation/Rifle/Reloading_Montage.Reloading_Montage"
    (:`then`
      (set `/Game/Blueprints/Weapons/BP_BaseWeapon.IsReloading` true _currentweaponbp))
    (:`OnCompleted`
      (set `/Game/Blueprints/Weapons/BP_BaseWeapon.IsReloading` false _currentweaponbp)
      (`/Game/Blueprints/Weapons/BP_BaseWeapon.Reload` _currentweaponbp))))

(event `self.ReceiveTick`
  (params (DeltaSeconds :type "Float (single-precision)"))
  (bind (_returnvalue_roll _returnvalue_pitch _returnvalue_yaw) (`KismetMathLibrary.BreakRotator` (`self.GetControlRotation`)))
  (bind _returnvalue (`KismetMathLibrary.ClampAngle` _returnvalue_pitch -50.0 50.0))
  ; Event Tick
  (`Controller.SetControlRotation` (`GameplayStatics.GetPlayerController` 0) (`KismetMathLibrary.MakeRotator` _returnvalue_roll _returnvalue _returnvalue_yaw))
  (set `self.RealPitch` _returnvalue))

(event `EnhancedInput|/Game/Character/Input/IA_Move`
  (params (ActionValue :type "Vector2D Structure") (ElapsedSeconds :type "Float (double-precision)") (TriggeredSeconds :type "Float (double-precision)") (InputAction :type "InputAction Object Reference" :default "/Game/Character/Input/IA_Move.IA_Move"))
  (bind (_returnvalue_roll _returnvalue_pitch _returnvalue_yaw) (`KismetMathLibrary.BreakRotator` (`self.GetControlRotation`)))
  ; IA_Move
  (:`Triggered`
    (`self.AddMovementInput` (`KismetMathLibrary.GetForwardVector` (`KismetMathLibrary.MakeRotator` 0.0 0.0 _returnvalue_yaw)) ActionValue_X)
    (`self.AddMovementInput` (`KismetMathLibrary.GetRightVector` (`self.GetControlRotation`)) ActionValue_Y)))

(event `EnhancedInput|/Game/Character/Input/IA_Look`
  (params (ActionValue :type "Vector2D Structure") (ElapsedSeconds :type "Float (double-precision)") (TriggeredSeconds :type "Float (double-precision)") (InputAction :type "InputAction Object Reference" :default "/Game/Character/Input/IA_Look.IA_Look"))
  ; IA_Look
  (:`Triggered`
    (`self.AddControllerYawInput` ActionValue_X)
    (bind _result (`/Engine/EditorBlueprintResources/StandardMacros.NegateFloat` ActionValue_Y)
      (:`  `
        (`self.AddControllerPitchInput` _result)))))

(event `EnhancedInput|/Game/Character/Input/IA_Sprint`
  (params (ActionValue :type Boolean) (ElapsedSeconds :type "Float (double-precision)") (TriggeredSeconds :type "Float (double-precision)") (InputAction :type "InputAction Object Reference" :default "/Game/Character/Input/IA_Sprint.IA_Sprint"))
  ; Sprint
  (:`Started`
    (if (not (`self.IsAiming`))
      (`self.Sprint`)))
  (:`Completed`
    (`self.Walk`)))

(event `EnhancedInput|/Game/Character/Input/IA_Aim`
  (params (ActionValue :type Boolean) (ElapsedSeconds :type "Float (double-precision)") (TriggeredSeconds :type "Float (double-precision)") (InputAction :type "InputAction Object Reference" :default "/Game/Character/Input/IA_Aim.IA_Aim"))
  (bind _charactermovement (`self.CharacterMovement`))
  (bind _charactermovement_2 (`self.CharacterMovement`))
  ; Aim
  (:`Started`
    (set `CharacterMovementComponent.bOrientRotationToMovement` false _charactermovement_2)
    (set `CharacterMovementComponent.bUseControllerDesiredRotation` true _charactermovement_2)
    (`self.Walk`)
    (set `self.IsAiming` true)
    (`Widget.SetVisibility` (`self.AimWidget`) "Visible")
    (bind (_direction _newtrack_0) (`Timeline|Timeline` :!label _label)
      (:`Update`
        (set `SpringArmComponent.TargetArmLength` (`KismetMathLibrary.Lerp` 200.0 100.0 _newtrack_0) (`self.SpringArm`)))))
  (:`Completed`
    (set `CharacterMovementComponent.bOrientRotationToMovement` true _charactermovement)
    (set `CharacterMovementComponent.bUseControllerDesiredRotation` false _charactermovement)
    (set `self.IsAiming` false)
    (`Widget.SetVisibility` (`self.AimWidget`) "Hidden")
    (goto _label :!via `Reverse`)))

(event `EnhancedInput|/Game/Character/Input/IA_Switch_Weapon`
  (params (ActionValue :type "Float (double-precision)") (ElapsedSeconds :type "Float (double-precision)") (TriggeredSeconds :type "Float (double-precision)") (InputAction :type "InputAction Object Reference" :default "/Game/Character/Input/IA_Switch_Weapon.IA_Switch_Weapon"))
  (bind _returnvalue (enumcount `/Game/ENUM/E_WeaponType`))
  ; Switch Weapon
  (:`Triggered`
    (switch `string` (`KismetStringLibrary.Conv_IntToString` (`KismetMathLibrary.FTrunc` ActionValue))
      (:`-1`
        (bind _output_get (set `self.CurrentWeaponIndex` (mod (+ (- (`self.CurrentWeaponIndex`) 1) _returnvalue) _returnvalue)))
        (`self.Switch Weapon` _output_get))
      (:`1`
        (bind _output_get_2 (set `self.CurrentWeaponIndex` (mod (+ (`self.CurrentWeaponIndex`) 1) (enumcount `/Game/ENUM/E_WeaponType`))))
        (`self.Switch Weapon` _output_get_2)))
    (`KismetSystemLibrary.PrintString` (`|GetEnumeratorNameAsString` (`self.CurrentWeapon`)))))

(event `EnhancedInput|/Game/Character/Input/IA_Shoot`
  (params (ActionValue :type Boolean) (ElapsedSeconds :type "Float (double-precision)") (TriggeredSeconds :type "Float (double-precision)") (InputAction :type "InputAction Object Reference" :default "/Game/Character/Input/IA_Shoot.IA_Shoot"))
  (bind _currentweaponbp (`self.CurrentWeaponBP`))
  (:`Started`
    (`/Engine/EditorBlueprintResources/StandardMacros.IsValid` _currentweaponbp
      (:`Is Valid`
        (if (`self.IsAiming`)
          (`/Game/Blueprints/Weapons/BP_BaseWeapon.Shoot` _currentweaponbp))))))

(event `EnhancedInput|/Game/Character/Input/IA_Reload`
  (params (ActionValue :type Boolean) (ElapsedSeconds :type "Float (double-precision)") (TriggeredSeconds :type "Float (double-precision)") (InputAction :type "InputAction Object Reference" :default "/Game/Character/Input/IA_Reload.IA_Reload"))
  (:`Triggered`
    (`self.ReloadGun`)))

(fn `Sprint`
  (set `CharacterMovementComponent.MaxWalkSpeed` 600.0 (`self.CharacterMovement`))
  (set `self.IsSprinting` true))

(fn `Switch Weapon`
  (params (`Weapon Index` :type Integer))
  (bind _currentweaponbp (`self.CurrentWeaponBP`))
  (bind _currentweaponbp_2 (`self.CurrentWeaponBP`))
  (switch `string` (`KismetStringLibrary.Conv_IntToString` `Weapon Index`)
    (:`0`
      (set `self.CurrentWeapon` "NewEnumerator0")
      (`/Engine/EditorBlueprintResources/StandardMacros.IsValid` _currentweaponbp_2
        (:`Is Valid`
          (`self.K2_DestroyActor` _currentweaponbp_2))
        (:`Is Not Valid`
          _))
      (bind _returnvalue (`|SpawnActorFromClass` "/Game/Blueprints/Weapons/BP_Pistol.BP_Pistol_C" (`self.GetTransform`) "Undefined" "MultiplyWithRoot" null null))
      (bind _output_get (set `self.CurrentWeaponBP` _returnvalue))
      (`self.K2_AttachToComponent` _output_get (`self.Mesh`) "Rifle_Idle_Socket" "SnapToTarget" "SnapToTarget" "SnapToTarget" true))
    (:`1`
      (set `self.CurrentWeapon` "NewEnumerator1")
      (`/Engine/EditorBlueprintResources/StandardMacros.IsValid` _currentweaponbp
        (:`Is Valid`
          (`self.K2_DestroyActor` _currentweaponbp))
        (:`Is Not Valid`
          _))
      (bind _returnvalue_2 (`|SpawnActorFromClass` "/Game/Blueprints/Weapons/BP_Rifle.BP_Rifle_C" (`self.GetTransform`) "Undefined" "MultiplyWithRoot" null null))
      (bind _output_get_2 (set `self.CurrentWeaponBP` _returnvalue_2))
      (`self.K2_AttachToComponent` _output_get_2 (`self.Mesh`) "Rifle_Idle_Socket" "SnapToTarget" "SnapToTarget" "SnapToTarget" true))))

(fn `UserConstructionScript`)

(fn `Walk`
  (set `CharacterMovementComponent.MaxWalkSpeed` 400.0 (`self.CharacterMovement`))
  (set `self.IsSprinting` false))